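; Pawn that moves forward on its own, trailing a snake-like chain of BP_Part actors.
; On BeginPlay it resets its transform and spawns the parts in a line spaced by Gap along negative X.
; Each Tick it offsets itself and the first part along its forward vector by Speed.
; Every other part follows the one ahead with constant-rate VInterpTo, using Speed divided by MovementFactor.
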(event `self.ReceiveBeginPlay`
  (`self.Spawn`))

(event `self.ReceiveTick`
  (params (DeltaSeconds :type "Float (single-precision)"))
  (`self.UpdateHeadLocation`)
  (`self.UpdatePartsLocation`))

(fn `Spawn`
  (locals (Location :type "Vector Structure"))
  (`self.K2_SetActorLocationAndRotation` (0.0 0.0 0.0) (struct) false true)
  (for _ (range (`self.PartsNum`))
    (bind _returnvalue (`|SpawnActorFromClass` "/Game/BP_Part.BP_Part_C" (`KismetMathLibrary.MakeTransform` (`local.Location`)) "Undefined" "OverrideRootScale" null null))
    (`KismetArrayLibrary.Array_Add` (`self.Parts`) _returnvalue)
    (set `local.Location` (- (`local.Location`) (`KismetMathLibrary.MakeVector` (`self.Gap`))))))

(fn `UpdateHeadLocation`
  (locals (Delta :type "Vector Structure"))
  (bind _output_get (set `local.Delta` (* (* (`GameplayStatics.GetWorldDeltaSeconds`) (`self.Speed`)) (`self.GetActorForwardVector`))))
  (`self.K2_AddActorWorldOffset` _output_get false true)
  (`self.K2_AddActorWorldOffset` (`|GetArrayItem` (`self.Parts`)) (`local.Delta`) false true))

(fn `UpdatePartsLocation`
  (locals (Index :type Integer) (CurrentLocation :type "Vector Structure" :default (0.0 0.0 0.0)) (TargetLocation :type "Vector Structure" :default (0.0 0.0 0.0)))
  (for _index (range 1 (+ (`KismetArrayLibrary.Array_LastIndex` (`self.Parts`)) 1))
    (set `local.Index` _index)
    (set `local.CurrentLocation` (`self.K2_GetActorLocation` (`|GetArrayItem` (`self.Parts`) (`local.Index`))))
    (set `local.TargetLocation` (`self.K2_GetActorLocation` (`|GetArrayItem` (`self.Parts`) (- (`local.Index`) 1))))
    (`self.K2_SetActorLocation` (`|GetArrayItem` (`self.Parts`) (`local.Index`)) (`KismetMathLibrary.VInterpTo_Constant` (`local.CurrentLocation`) (`local.TargetLocation`) (`GameplayStatics.GetWorldDeltaSeconds`) (/ (`self.Speed`) (`self.MovementFactor`))) false true)))

(fn `UserConstructionScript`)