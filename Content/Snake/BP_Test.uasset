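; Snake prototype actor whose body is a chain of Instanced Static Mesh segments, laid out in a line by the construction script.
; Each tick the head instance turns at a constant rate toward the point under the mouse cursor and moves forward, shifting the spring arm with it.
; Each following segment interpolates its yaw and XY location toward the segment ahead, at a rate based on speed and a movement factor.
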(event `self.ReceiveBeginPlay`
  (bind _output_get (set `self.PlayerController` (`GameplayStatics.GetPlayerController` 0)))
  (set `PlayerController.bShowMouseCursor` false _output_get)
  (`SceneComponent.SetAbsolute` (`self.ISM`) true true true))

(event `self.ReceiveTick`
  (params (DeltaSeconds :type "Float (single-precision)"))
  (set `self.Delta Seconds` DeltaSeconds)
  (`self.UpdateHead`)
  (`self.UpdateInstnaces`))

(fn `AddInstanceOffset`
  (params (Index :type Integer) (Offset :type "Vector Structure") (World :type Boolean) (Teleport :type Boolean))
  (bind _outinstancetransform (`InstancedStaticMeshComponent.GetInstanceTransform` (`self.ISM`) (`local.Index`) (`local.World`)))
  (`InstancedStaticMeshComponent.UpdateInstanceTransform` (`self.ISM`) (`local.Index`) (`KismetMathLibrary.MakeTransform` (+ Offset (.location _outinstancetransform)) (.rotation _outinstancetransform) (.scale _outinstancetransform)) (`local.World`) true (`local.Teleport`)))

(fn `GetInstanceForwardVector`
  (params (Index :type Integer))
  (returns (ForwardVector :type "Vector Structure"))
  (return (`KismetMathLibrary.GetForwardVector` (.rotation (`InstancedStaticMeshComponent.GetInstanceTransform` (`self.ISM`) (`local.Index`) true)))))

(fn `GetInstanceLocation`
  (params (Index :type Integer))
  (returns (Location :type "Vector Structure"))
  (return (.location (`InstancedStaticMeshComponent.GetInstanceTransform` (`self.ISM`) (`local.Index`) true))))

(fn `GetInstanceRotation`
  (params (Index :type Integer))
  (returns (Rotation :type "Rotator Structure"))
  (return (.rotation (`InstancedStaticMeshComponent.GetInstanceTransform` (`self.ISM`) (`local.Index`) true))))

(fn `GetInstanceScale`
  (params (Index :type Integer))
  (returns (Scale :type "Vector Structure"))
  (return (.scale (`InstancedStaticMeshComponent.GetInstanceTransform` (`self.ISM`) (`local.Index`) true))))

(fn `GetLastInstanceIndex`
  (returns (Index :type Integer))
  (return (- (`InstancedStaticMeshComponent.GetInstanceCount` (`self.ISM`)) 1)))

(fn `SetInstanceLocation`
  (params (Index :type Integer) (Location :type "Vector Structure") (World :type Boolean) (Teleport :type Boolean))
  (locals (CurrentRotation :type "Rotator Structure") (CurrentScale :type "Vector Structure"))
  (set `local.CurrentRotation` (`self.GetInstanceRotation` (`local.Index`)))
  (set `local.CurrentScale` (`self.GetInstanceScale` (`local.Index`)))
  (`InstancedStaticMeshComponent.UpdateInstanceTransform` (`self.ISM`) (`local.Index`) (`KismetMathLibrary.MakeTransform` (`local.Location`) (`local.CurrentRotation`) (`local.CurrentScale`)) (`local.World`) true (`local.Teleport`)))

(fn `SetInstanceRotation`
  (params (Index :type Integer) (Rotation :type "Rotator Structure") (World :type Boolean) (Teleport :type Boolean))
  (locals (CurrentLocation :type "Vector Structure") (CurrentScale :type "Vector Structure"))
  (set `local.CurrentLocation` (`self.GetInstanceLocation` (`local.Index`)))
  (set `local.CurrentScale` (`self.GetInstanceScale` (`local.Index`)))
  (`InstancedStaticMeshComponent.UpdateInstanceTransform` (`self.ISM`) (`local.Index`) (`KismetMathLibrary.MakeTransform` (`local.CurrentLocation`) (`local.Rotation`) (`local.CurrentScale`)) (`local.World`) true (`local.Teleport`)))

(fn `UpdateHead`
  (locals (Location :type "Vector Structure") (CurrentRotation :type "Rotator Structure") (NewRotation :type "Rotator Structure"))
  (bind (_returnvalue_x _returnvalue_y) (`KismetMathLibrary.BreakVector` (* (* (`self.Speed`) (`self.Delta Seconds`)) (`self.GetInstanceForwardVector` 0))))
  (set `local.Location` (`self.GetInstanceLocation` 0))
  (set `local.CurrentRotation` (`self.GetInstanceRotation` 0))
  (set `local.NewRotation` (`KismetMathLibrary.RInterpTo_Constant` (`local.CurrentRotation`) (`KismetMathLibrary.FindLookAtRotation` (`local.Location`) (`.Location` (`GameplayStatics.BreakHitResult` (`PlayerController.GetHitResultUnderCursorByChannel` (`self.PlayerController`) "TraceTypeQuery1" true)))) (`self.Delta Seconds`) (`self.TurnSpeed`)))
  (`self.SetInstanceRotation` 0 (`local.NewRotation`) true true)
  (`self.AddInstanceOffset` 0 (`KismetMathLibrary.MakeVector` _returnvalue_x _returnvalue_y) true true)
  (`SceneComponent.K2_AddWorldOffset` (`self.SpringArm`) (`KismetMathLibrary.MakeVector` _returnvalue_x _returnvalue_y) false true))

(fn `UpdateInstnaces`
  (locals (Index :type Integer) (CurrentLocation :type "Vector Structure") (TargetLocation :type "Vector Structure") (CurrentRotation :type "Rotator Structure") (TargetRotation :type "Rotator Structure"))
  (bind (_returnvalue_roll _returnvalue_pitch _returnvalue_yaw) (`KismetMathLibrary.BreakRotator` (`KismetMathLibrary.RInterpTo_Constant` (`local.CurrentRotation`) (`local.TargetRotation`) (`self.Delta Seconds`) (/ (`self.Speed`) (`self.MovementFactor`)))))
  (bind (_returnvalue_x _returnvalue_y) (`KismetMathLibrary.BreakVector` (`KismetMathLibrary.VInterpTo` (`local.CurrentLocation`) (`local.TargetLocation`) (`self.Delta Seconds`) (/ (`self.Speed`) (`self.MovementFactor`)))))
  (for _index (range 1 (+ (`self.GetLastInstanceIndex`) 1))
    (set `local.Index` _index)
    (set `local.CurrentLocation` (`self.GetInstanceLocation` (`local.Index`)))
    (set `local.CurrentRotation` (`self.GetInstanceRotation` (`local.Index`)))
    (set `local.TargetRotation` (`self.GetInstanceRotation` (- (`local.Index`) 1)))
    (`self.SetInstanceRotation` (`local.Index`) (`KismetMathLibrary.MakeRotator` 0.0 0.0 _returnvalue_yaw) true true)
    (set `local.TargetLocation` (`self.GetInstanceLocation` (- (`local.Index`) 1)))
    (`self.SetInstanceLocation` (`local.Index`) (`KismetMathLibrary.MakeVector` _returnvalue_x _returnvalue_y) true true)))

(fn `UserConstructionScript`
  (locals (Location :type "Vector Structure" :default (0.0 0.0 0.0)) (Index :type Integer))
  (`self.K2_SetActorTransform` (`KismetMathLibrary.MakeTransform` (0.0 0.0 0.0) (struct)) false true)
  (`StaticMeshComponent.SetStaticMesh` (`self.ISM`) (`self.Mesh`))
  (`PrimitiveComponent.SetMaterial` (`self.ISM`) 0 (`self.Material`))
  (for _index (range (`self.ISMLength`))
    (set `local.Index` _index)
    (`InstancedStaticMeshComponent.AddInstance` (`self.ISM`) (`KismetMathLibrary.MakeTransform` (`local.Location`)) true)
    (set `local.Location` (- (`local.Location`) (`KismetMathLibrary.MakeVector` (`self.Gap`))))))